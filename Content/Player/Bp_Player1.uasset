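; Player 1 Blueprint that links the player's component data to the UI for points and card display.
; Shortly after BeginPlay it registers itself with the UI, then pushes the component's points to it every Tick.
; ShowCards looks up card indices for the saved piece's role and passes the first two to the UI, while HideCards hides them.
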(event `self.ReceiveBeginPlay`
  (`KismetSystemLibrary.Delay` 0.5)
  (set `/Game/Player/Bp_WidgetPlayer.Player1_ref` self (`self.UI`)))

(event `self.ReceiveTick`
  (params (DeltaSeconds :type "Float (single-precision)"))
  (if (`KismetSystemLibrary.IsValid` (`self.UI`))
    (`/Game/Player/Bp_WidgetPlayer.SetPoints` (`self.UI`) (`KismetTextLibrary.Conv_IntToText` (`PlayerComponent.Points` (`self.PlayerComponent`))))))

(event `self.ShowCards`
  (bind _savedpiece (`self.SavedPiece`))
  (`/Engine/EditorBlueprintResources/StandardMacros.IsValid` _savedpiece
    (:`Is Valid`
      (bind _returnvalue (`PlayerComponent.GetCardIndexOfRole` (`self.PlayerComponent`) (`.RoleName` (break `Role` (`CPP_Piece.PieceRole` _savedpiece)))))
      (if (`KismetArrayLibrary.Array_IsNotEmpty` _returnvalue)
        (`/Game/Player/Bp_WidgetPlayer.ShowCards` (`self.UI`) (`|GetArrayItem` _returnvalue) (`|GetArrayItem` _returnvalue 1))))))

(event `self.HideCards`
  (`/Game/Player/Bp_WidgetPlayer.Hide Cards` (`self.UI`)))

(fn `UserConstructionScript`)