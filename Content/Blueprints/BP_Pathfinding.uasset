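; Pathfinding test Blueprint that visualizes which board tiles are reachable from a start position within a step limit.
; After a short delay on BeginPlay, it runs a hardcoded four-direction search on the Board.
; Each returned tile gets a dynamic M_PathfindMarking material, with color scaled down as path cost rises and zero-cost tiles given a fixed color.
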(event `self.ReceiveBeginPlay`
  (`KismetSystemLibrary.Delay` 3.0)
  (`self.Run Pathfinding` (make `2DVectorInt` 3 4) (`|MakeArray` (make `2DVectorInt` 1) (make `2DVectorInt` -1) (make `2DVectorInt` 0 1) (make `2DVectorInt` 0 -1)) 4))

(fn `Run Pathfinding`
  (params (`Start Position` :type "2DVectorInt Structure") (`Movement Options` :type "Array of 2DVectorInt Structure") (Steps :type Integer))
  (bind (_x _y) (break `2DVectorInt` `Start Position`))
  (bind _returnvalue (`KismetMathLibrary.Conv_IntToDouble` (+ (`local.Steps`) 1)))
  ;[1 1 1 1 36] Check Start Position Validity
  (bind _returnvalue_2 (`CPP_Board.GetTileAt` (`self.Board`) _x _y))
  (`/Engine/EditorBlueprintResources/StandardMacros.IsValid` _returnvalue_2
    (:`Is Valid`
      ;[1 1 1 1 36] Run Pathfinding Function and Update Material Color for Reachable Tiles
      (bind _returnvalue_3 (`self.RunPathfinding` `Start Position` `Movement Options` (`self.Board`) Steps))
      (for _array_element _returnvalue_3
        (bind (_x_2 _y_2) (break `2DVectorInt` (`CPP_AlgorithmPath.Position` _array_element)))
        (bind _returnvalue_4 (`CPP_Board.GetTileAt` (`self.Board`) _x_2 _y_2))
        (`/Engine/EditorBlueprintResources/StandardMacros.IsValid` _returnvalue_4
          (:`Is Valid`
            (bind _returnvalue_5 (`KismetMaterialLibrary.CreateDynamicMaterialInstance` "/Game/Resources/Materials/M_PathfindMarking.M_PathfindMarking"))
            (bind _returnvalue_6 (`MaterialInstanceDynamic.K2_GetVectorParameterValue` _returnvalue_5 "Color"))
            (bind _pathcost (`CPP_AlgorithmPath.PathCost` _array_element))
            (if (> _pathcost 0)
              (`MaterialInstanceDynamic.SetVectorParameterValue` _returnvalue_5 "Color" (* (/ (- _returnvalue (`KismetMathLibrary.Conv_IntToDouble` _pathcost)) _returnvalue) _returnvalue_6))
              (else
                (`MaterialInstanceDynamic.SetVectorParameterValue` _returnvalue_5 "Color" (struct :`G` 0.5 :`B` 0.25 :`A` 1.0))))
            (`PrimitiveComponent.SetMaterial` (`CPP_Tile.Mesh` _returnvalue_4) 0 _returnvalue_5)))))))

(fn `UserConstructionScript`)