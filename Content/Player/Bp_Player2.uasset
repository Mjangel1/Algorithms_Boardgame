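; Player 2 actor Blueprint that links the player's component data to its UI.
; After a short delay on BeginPlay it registers itself with the UI, then pushes the component's points to the UI every tick.
; ShowCards looks up the card indices for the saved piece's role and shows two cards in the UI, while HideCards hides them.
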(event `self.ReceiveBeginPlay`
  (`KismetSystemLibrary.Delay` 0.5)
  (set `/Game/Player/Bp_WidgetPlayer2.Player2_ref` self (`self.UI`)))

(event `self.ReceiveTick`
  (params (DeltaSeconds :type "Float (single-precision)"))
  (if (`KismetSystemLibrary.IsValid` (`self.UI`))
    (`/Game/Player/Bp_WidgetPlayer2.SetPoints` (`self.UI`) (`KismetTextLibrary.Conv_IntToText` (`PlayerComponent.Points` (`self.PlayerComponent`))))))

(event `self.ShowCards`
  (bind _savedpiece (`self.SavedPiece`))
  (`/Engine/EditorBlueprintResources/StandardMacros.IsValid` _savedpiece
    (:`Is Valid`
      (bind _returnvalue (`PlayerComponent.GetCardIndexOfRole` (`self.PlayerComponent`) (`.RoleName` (break `Role` (`CPP_Piece.PieceRole` _savedpiece)))))
      (if (`KismetArrayLibrary.Array_IsNotEmpty` _returnvalue)
        (`/Game/Player/Bp_WidgetPlayer2.ShowCards` (`self.UI`) (`|GetArrayItem` _returnvalue) (`|GetArrayItem` _returnvalue 1))))))

(event `self.HideCards`
  (`/Game/Player/Bp_WidgetPlayer2.HideCards` (`self.UI`)))

(fn `UserConstructionScript`)